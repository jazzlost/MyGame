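; Blueprint function library that shares named user widgets and toggles the options screen in a 2D side-scroller project.
; Add, get and set helpers forward to widget storage on the 2DSideScrollerGameMode, printing a message if the game mode cast fails.
; SetOptionWidgetVisibility looks up the Myshow_option widget and swaps it with a valid parent widget, adding one to the viewport and removing and hiding the other.
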(fn `AddUserWidget`
  (params (UserWidget :type "UserWidget Object Reference") (WidgetName :type Name))
  (bind _as2dside_scroller_game_mode (`self.GetMyGameMode` null))
  (`/Game/2DSideScrollerBP/Blueprints/2DSideScrollerGameMode.AddUserWidget` _as2dside_scroller_game_mode UserWidget WidgetName)
  (return))

(fn `GetMyGameMode`
  (returns (`As2DSide Scroller Game Mode` :type "/Game/2DSideScrollerBP/Blueprints/2DSideScrollerGameMode Object Reference"))
  (bind _as2dside_scroller_game_mode (cast `/Game/2DSideScrollerBP/Blueprints/2DSideScrollerGameMode` (`GameplayStatics.GetGameMode` null))
    (:`then`
      (return _as2dside_scroller_game_mode))
    (:`CastFailed`
      (`KismetSystemLibrary.PrintString` null "Game Mode Not 2DSideScrollerGameMode!"))))

(fn `GetUserWidget`
  (params (WidgetName :type Name))
  (returns (UserWidget :type "UserWidget Object Reference"))
  (bind _as2dside_scroller_game_mode (`self.GetMyGameMode` null))
  (bind _userwidget (`/Game/2DSideScrollerBP/Blueprints/2DSideScrollerGameMode.GetUserWidget` _as2dside_scroller_game_mode WidgetName))
  (`/Engine/EditorBlueprintResources/StandardMacros.IsValid` _userwidget
    (:`Is Valid`
      (return _userwidget))))

(fn `SetOptionWidgetVisibility`
  (params (bIsVisible :type Boolean) (ParentWidget :type "UserWidget Object Reference"))
  (`/Engine/EditorBlueprintResources/StandardMacros.IsValid` ParentWidget
    (:`Is Valid`
      (bind _userwidget (`self.GetUserWidget` null "Myshow_option"))
      (if bIsVisible
        (`Widget.RemoveFromParent` ParentWidget)
        (`Widget.SetVisibility` ParentWidget "Hidden")
        (`Widget.SetVisibility` _userwidget "Visible")
        (`UserWidget.AddToViewport` _userwidget 0)
        (else
          (`Widget.RemoveFromParent` _userwidget)
          (`Widget.SetVisibility` ParentWidget "Visible")
          (`Widget.SetVisibility` _userwidget "Hidden")
          (`UserWidget.AddToViewport` ParentWidget 0))))
    (:`Is Not Valid`
      (return))))

(fn `SetUserWidget`
  (params (WidgetName :type Name) (UserWidget :type "UserWidget Object Reference"))
  (bind _as2dside_scroller_game_mode (`self.GetMyGameMode` null))
  (`/Game/2DSideScrollerBP/Blueprints/2DSideScrollerGameMode.SetUserWidget` _as2dside_scroller_game_mode WidgetName UserWidget)
  (return))