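; ReturnButton is a UI button that handles returning to the widget named by ReturnWidgetName.
; InitButton binds its click, hover and unhover events and caches the first player controller.
; A click passes that name to SetUserWidgetVisibility and posts the Wwise Back sound event on the controller.
; Hovering enlarges the button through its render scale, and unhovering restores it.
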(event `InitButton`
  (bind _returnvalue (`GameplayStatics.GetPlayerController` 0))
  ;[1 1 1] Init
  (add `self.OnClicked` (delegate `OnClickedButton`))
  (add `self.OnHovered` (delegate `OnHoveredButton`))
  (add `self.OnUnhovered` (delegate `OnUnhoveredButton`))
  (`/Engine/EditorBlueprintResources/StandardMacros.IsValid` _returnvalue
    (:`Is Valid`
      (set `self.PlayerController` _returnvalue))))

(event `OnClickedButton`
  (`/Game/Blueprints/MyShowFunctionLibrary.SetUserWidgetVisibility` (`self.ReturnWidgetName`))
  (`AkGameplayStatics.PostEvent` "/Game/MusicGame/Back.Back" (`self.PlayerController`)))

(event `OnHoveredButton`
  (`self.SetRenderScale` (1.2 1.2)))

(event `OnUnhoveredButton`
  (`self.SetRenderScale` (1.0 1.0)))