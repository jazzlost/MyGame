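; Options button that opens the options menu, with a Wwise click sound and render-scale feedback for hover and press.
; InitButton binds the button events and creates a hidden Myshow_option widget once, guarded by a flag on 2DSideScrollerGameMode.
; Clicking registers the parent widget as OptionReturnWidget in a name-based widget lookup, then calls SetOptionWidgetVisibility to show the options with that parent.
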(event `InitButton`
  (bind _returnvalue (`GameplayStatics.GetPlayerController` 0))
  ;[1 1 1] Event Bind
  (`self.InitOptionWidget`)
  (add `self.OnClicked` (delegate `OnButtonClick`))
  (add `self.OnPressed` (delegate `OnPressedButton`))
  (add `self.OnReleased` (delegate `OnReleasedButton`))
  (add `self.OnHovered` (delegate `OnHoveredButton`))
  (add `self.OnUnhovered` (delegate `OnUnhoveredButton`))
  (`/Engine/EditorBlueprintResources/StandardMacros.IsValid` _returnvalue
    (:`Is Valid`
      (set `self.PlayerController` _returnvalue))))

(event `OnButtonClick`
  ;[1 1 1] Button Event
  (`AkGameplayStatics.PostEvent` "/Game/MusicGame/option.option" (`self.PlayerController`))
  (bind _userwidget (`/Game/Blueprints/MyShowFunctionLibrary.GetUserWidget` (`self.ParentWidgetName`)))
  (`/Game/Blueprints/MyShowFunctionLibrary.SetUserWidget` "OptionReturnWidget" _userwidget)
  (`/Game/Blueprints/MyShowFunctionLibrary.SetOptionWidgetVisibility` true _userwidget))

(event `OnPressedButton`
  ;[1 1 1] Button Event
  (`self.SetRenderScale` (0.5 0.5)))

(event `OnReleasedButton`
  ;[1 1 1] Button Event
  (`self.SetRenderScale` (0.3 0.3)))

(event `OnHoveredButton`
  ;[1 1 1] Button Event
  (`self.SetRenderScale` (0.4 0.4)))

(event `OnUnhoveredButton`
  ;[1 1 1] Button Event
  (`self.SetRenderScale` (0.3 0.3)))

(fn `GetCanCreateOptionWidget`
  (returns (bCanCreateOptionWidget :type Boolean))
  (bind _as2dside_scroller_game_mode (cast `/Game/2DSideScrollerBP/Blueprints/2DSideScrollerGameMode` (`GameplayStatics.GetGameMode`)))
  (return (`/Game/2DSideScrollerBP/Blueprints/2DSideScrollerGameMode.bCanCreateOptionWidget` _as2dside_scroller_game_mode)))

(fn `InitOptionWidget`
  (bind _bcancreateoptionwidget (`self.GetCanCreateOptionWidget`))
  (if _bcancreateoptionwidget
    (bind _returnvalue (`|CreateWidget` "/Game/Myshow_option.Myshow_option_C"))
    (`/Game/Blueprints/MyShowFunctionLibrary.SetUserWidget` "Myshow_option" _returnvalue)
    (`self.SetVisibility` _returnvalue "Hidden")
    (`self.SetCanCreateOptionWidget` false)
    (else
      (return))))

(fn `SetCanCreateOptionWidget`
  (params (IsFirstTime :type Boolean))
  (bind _as2dside_scroller_game_mode (cast `/Game/2DSideScrollerBP/Blueprints/2DSideScrollerGameMode` (`GameplayStatics.GetGameMode`)))
  (set `/Game/2DSideScrollerBP/Blueprints/2DSideScrollerGameMode.bCanCreateOptionWidget` IsFirstTime _as2dside_scroller_game_mode)
  (return))